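; A floor-style button actor that latches down when an actor overlaps it and stays pressed until its ToggleOff event is called.
; BeginPlay creates a dynamic material and caches the raised and depressed positions.
; A DoOnce gates the overlap, which sets Toggled, plays a press sound and runs a timeline driving both actor height and the material's Toggle light parameter.
; ToggleOff resets the gate, plays a reset sound and reverses the timeline.
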(event Custom|ToggleOff
  (Variables|Default|SetbToggled false)
  (Utilities|FlowControl|Sequence
    (:then_0
      (Utilities|FlowControl|DoOnce false) ; enters at Reset
    )
    (:then_1
      (Utilities|PlaySoundifExists (Variables|Default|GetResetSound))
      ;[0.4819 0.7394 1] Depress/raise button
      (bind _buttonpos (Timeline|SwitchTimeline Reverse)
        (:Update
          (Transformation|SetActorLocation (Math|Vector|Lerp(Vector) (Variables|Default|GetOrigPosition) (Variables|Default|GetDepressedPosition) _buttonpos) false false)
          ;[1 0.1979 0.1999] Turn button light on/off
          (Rendering|Material|SetScalarParameterValue (Variables|Default|GetMaterial) "Toggle" _buttonpos :!class /Script/Engine.MaterialInstanceDynamic))))))

(event EventBeginPlay
  ;[0.4001 0.7344 0.4579] Store button material and raised/depressed positions
  (bind _returnvalue (Rendering|Material|CreateDynamicMaterialInstance (Variables|Debug|GetStaticMeshComponent) 0 0 "None" :!class /Script/Engine.PrimitiveComponent))
  (Variables|Default|SetMaterial _returnvalue)
  (bind _output_get (Variables|Default|SetOrigPosition (Transformation|GetActorLocation)))
  (Variables|Default|SetDepressedPosition (- _output_get "0.000000,0.000000,5.000000")))

(event Collision|EventActorBeginOverlap
  (params (OtherActor :type Actor%20Object%20Reference))
  (Utilities|FlowControl|DoOnce false
    (:Completed
      (Variables|Default|SetbToggled true)
      (Utilities|PlaySoundifExists (Variables|Default|GetPressSound))
      ;[0.4819 0.7394 1] Depress/raise button
      (bind _buttonpos (Timeline|SwitchTimeline Play)
        (:Update
          (Transformation|SetActorLocation (Math|Vector|Lerp(Vector) (Variables|Default|GetOrigPosition) (Variables|Default|GetDepressedPosition) _buttonpos) false false)
          ;[1 0.1979 0.1999] Turn button light on/off
          (Rendering|Material|SetScalarParameterValue (Variables|Default|GetMaterial) "Toggle" _buttonpos :!class /Script/Engine.MaterialInstanceDynamic))))))

(fn ConstructionScript)