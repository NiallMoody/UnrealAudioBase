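; Floor button that checks the garden puzzle, sinking and rising on overlap with sounds and a retrigger guard.
; Each press counts toggled actors in Buttons; unless all are on, it resets them and plays a failure sound.
; When all are on, it lights Connectors with a delayed loop, plays success sounds, and moves the cathedral door and centre columns by timeline.
; Once the columns finish, it notifies the centre rings that the garden is solved.
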(event Collision|EventActorEndOverlap
  (params (OtherActor :type Actor%20Object%20Reference))
  ;[0.7093 0.4983 1] Depress/raise button
  (Utilities|PreventOverlapRetriggers) ; enters at Button Release In
)

(event Collision|EventActorBeginOverlap
  (params (OtherActor :type Actor%20Object%20Reference))
  (bind _cathedraldoor (Variables|Config|GetCathedralDoor))
  (bind _centrecolumns (Variables|Config|GetCentreColumns))
  (bind _returnvalue (Transformation|GetActorLocation _centrecolumns))
  (bind _returnvalue_2 (Transformation|GetActorLocation _cathedraldoor))
  (Variables|Default|SetNumToggled 0)
  (Utilities|FlowControl|Sequence
    (:then_0
      ;[0.7093 0.4983 1] Depress/raise button
      (Utilities|PreventOverlapRetriggers :!label _label
        (:Button%20Press%20Out
          (Utilities|PlaySoundifExistsSelf (Variables|Sounds|GetPressSound))
          (bind _buttonpos (Timeline|ButtonDepressTimeline Play)
            (:Update
              (Transformation|SetActorLocation (Math|Vector|Lerp(Vector) (Variables|Default|GetOrigPosition) (Variables|Default|GetDepressedPosition) _buttonpos) false false))
            (:Finished
              (goto _label Reset))))
        (:Button%20Release%20Out
          (Utilities|PlaySoundifExistsSelf (Variables|Sounds|GetReleaseSound))
          (Timeline|ButtonDepressTimeline Reverse))))
    (:then_1
      ;[0.5059 0.7143 1] Count pressed buttons
      (for _array_element (Variables|Config|GetButtons)
        (if (Variables|/Game/UnrealAudioBase/Blueprints/BP_IndividualButton.BP_IndividualButton_C|GetbToggled _array_element)
          (Math|Integer|IncrementInt (Variables|Default|GetNumToggled))))
      (if (== (Variables|Default|GetNumToggled) (Utilities|Array|Length (Variables|Config|GetButtons)))
        ;[0.2977 1 0.5863] If all buttons are lit, light connections...
        (bind _array_element_2 (Utilities|DelayedforEach (Variables|Config|GetConnectors) 0.25)
          (:Loop%20Body
            (Default|Toggleon _array_element_2))
          (:Completed
            ;[0.4578 0.6018 1] Play 'Puzzle Solved' sound...
            (Utilities|PlaySoundifExistsSelf (Variables|Sounds|GetPuzzleSolved))
            ;[0.7118 1 0.5475] Trigger centre columns sound...
            (Utilities|PlaySoundifExists (Variables|Sounds|GetCentreTowersSound) (Transformation|GetActorLocation (Variables|Config|GetCentreColumns)))
            (Utilities|FlowControl|Sequence
              (:then_0
                ;[1 0.4277 0.7468] Lower Cathedral Door
                (bind _doorypos (Timeline|CathedralDoorTimeline Play)
                  (:Update
                    (Transformation|SetActorLocation _cathedraldoor (Math|Vector|MakeVector (.x _returnvalue_2) (.y _returnvalue_2) _doorypos) false false))))
              (:then_1
                ;[1 0.5577 0.3343] Lower centre columns...
                (bind _columnsypos (Timeline|CentreColumnsTimeline Play)
                  (:Update
                    (Transformation|SetActorLocation _centrecolumns (Math|Vector|MakeVector (.x _returnvalue) (.y _returnvalue) _columnsypos) false false))
                  (:Finished
                    ;[0.3764 0.3244 1] And inform centre rings the garden puzzle is solved
                    (for _array_element_3 (Variables|Config|GetCentreRings)
                      (Default|GardenSolved _array_element_3))))))))
        (else
          ;[1 0.3122 0.3321] If not all buttons are lit, turn them all off/force restart...
          (for _array_element_4 (Variables|Config|GetButtons)
            (Default|ToggleOff _array_element_4))
          ;[1 0.1277 0.2656] And play 'Puzzle Failed' sound
          (Utilities|FlowControl|DoOnce false :!label _label_2
            (:Completed
              (Utilities|PlaySoundifExistsSelf (Variables|Sounds|GetPuzzleFailed))
              (Utilities|FlowControl|Delay 0.2)
              (goto _label_2 Reset))))))))

(event EventBeginPlay
  ;[0.1988 1 0.7677] Store button depressed/raised position
  (bind _output_get (Variables|Default|SetOrigPosition (Transformation|GetActorLocation)))
  (Variables|Default|SetDepressedPosition (- _output_get "0.000000,0.000000,5.000000")))

(fn ConstructionScript)