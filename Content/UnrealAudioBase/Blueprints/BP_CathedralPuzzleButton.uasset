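; Cathedral puzzle submit button that sinks when overlapped and rises on release, using a retrigger guard and timeline.
; On overlap it compares the Buttons' toggle states to the Solution array, requiring nine matches.
; Success lights Connections sequentially via a delayed loop, lowers the centre internal wall by timeline, then notifies CentreRings.
; Failure switches every puzzle button off and plays a fail sound, throttled by a DoOnce and short delay.
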(event Collision|EventActorEndOverlap
  (params (OtherActor :type Actor%20Object%20Reference))
  ;[0.7084 0.4969 1] Depress/raise button
  (Utilities|PreventOverlapRetriggers) ; enters at Button Release In
)

(event Collision|EventActorBeginOverlap
  (params (OtherActor :type Actor%20Object%20Reference))
  (bind _internalwall (Variables|Config|GetInternalWall))
  (bind _returnvalue (Transformation|GetActorLocation _internalwall))
  (Variables|Default|SetNumCorrect 0)
  (Utilities|FlowControl|Sequence
    (:then_0
      ;[0.7084 0.4969 1] Depress/raise button
      (Utilities|PreventOverlapRetriggers :!label _label
        (:Button%20Press%20Out
          (Utilities|PlaySoundifExistsSelf (Variables|Sounds|GetPressSound))
          (bind _buttonpos (Timeline|ButtonDepressTimeline Play)
            (:Update
              (Transformation|SetActorLocation (Math|Vector|Lerp(Vector) (Variables|Default|GetOrigPosition) (Variables|Default|GetDepressedPosition) _buttonpos) false false))
            (:Finished
              (goto _label Reset))))
        (:Button%20Release%20Out
          (Utilities|PlaySoundifExistsSelf (Variables|Sounds|GetReleaseSound))
          (Timeline|ButtonDepressTimeline Reverse))))
    (:then_1
      ;[0.4637 0.8277 1] Count correct button states
      (for (_array_element _array_index) (Variables|Config|GetButtons)
        (if (== (Variables|/Game/UnrealAudioBase/Blueprints/BP_IndividualButton.BP_IndividualButton_C|GetbToggled _array_element) (Utilities|Array|Get(acopy) (Variables|Config|GetSolution) _array_index))
          (Math|Integer|IncrementInt (Variables|Default|GetNumCorrect))))
      (if (== (Variables|Default|GetNumCorrect) 9)
        ;[0.2961 1 0.5906] If correct buttons are on, light connections...
        (bind _array_element_2 (Utilities|DelayedforEach (Variables|Config|GetConnections) 0.25)
          (:Loop%20Body
            (Default|Toggleon _array_element_2))
          (:Completed
            ;[0.4588 0.6 1] Play 'Puzzle Solved' sound...
            (Utilities|PlaySoundifExistsSelf (Variables|Sounds|GetPuzzleSolved))
            ;[0.7137 1 0.549] Play Centre Wall lowering sound...
            (Utilities|PlaySoundifExists (Variables|Sounds|GetCentreWallSound) (Transformation|GetActorLocation (Variables|Config|GetInternalWall)))
            ;[0.3589 0.9344 0.899] Lower Centre Internal Wall...
            (bind _wallypos (Timeline|InternalWallTimeline Play)
              (:Update
                (Transformation|SetActorLocation _internalwall (Math|Vector|MakeVector (.x _returnvalue) (.y _returnvalue) _wallypos) false false))
              (:Finished
                ;[1 0.3891 0.1981] And inform centre rings the puzzle is solved
                (for _array_element_3 (Variables|Config|GetCentreRings)
                  (Default|CathedralSolved _array_element_3))))))
        (else
          ;[1 0.314 0.3325] If buttons incorrect, reset all
          (for _array_element_4 (Variables|Config|GetButtons)
            (Default|ToggleOff _array_element_4))
          ;[1 0.1294 0.2667] And play 'Puzzle Failed' sound
          (Utilities|FlowControl|DoOnce false :!label _label_2
            (:Completed
              (Utilities|PlaySoundifExistsSelf (Variables|Sounds|GetPuzzleFailed))
              (Utilities|FlowControl|Delay 0.2)
              (goto _label_2 Reset))))))))

(event EventBeginPlay
  ;[1 0.3767 0.2021] Store button depressed/raised positions
  (bind _output_get (Variables|Default|SetOrigPosition (Transformation|GetActorLocation)))
  (Variables|Default|SetDepressedPosition (- _output_get "0.000000,0.000000,5.000000")))

(fn ConstructionScript)