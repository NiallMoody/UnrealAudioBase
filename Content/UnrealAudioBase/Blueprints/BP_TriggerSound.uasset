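; BP_TriggerSound is a trigger actor that plays an assigned sound when the player character overlaps it.
; On begin overlap it confirms the actor is the player and that Sound is valid.
; A OnceOnly flag routes through a DoOnce node to limit playback to a single trigger.
; The sound plays at the player's location, as an approximation rather than an exact source position.
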(event Collision|EventActorBeginOverlap
  (params (OtherActor :type Actor%20Object%20Reference))
  (bind _returnvalue (Game|GetPlayerCharacter 0))
  (bind _sound (Variables|Default|GetSound))
  ;[1 0.2471 0.2809] Check sound exists
  (if (== OtherActor _returnvalue)
    (if (Utilities|IsValid _sound)
      ;[1 0.4819 0.3395] Trigger just one time if Once Only is true
      (if (Variables|Default|GetbOnceOnly)
        (Utilities|FlowControl|DoOnce false
          (:Completed
            _)))
      (Audio|PlaySoundatLocation _sound (Transformation|GetActorLocation _returnvalue) "0, 0, 0" 1.0 1.0 0.0 0 0 0 0))))

(fn ConstructionScript)