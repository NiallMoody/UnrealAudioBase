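; BP_EndTrigger is a trigger actor that runs the game's ending sequence once the player overlaps it.
; It disables player input, blends the view to a static EndCamera looking up through spinning rings, and waits for the blend to finish.
; It then plays an ending sound and fades the screen to white while a timeline animates the camera's FOV.
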(event Collision|EventActorBeginOverlap
  (params (OtherActor :type Actor%20Object%20Reference))
  (bind _returnvalue (Game|GetPlayerController 0))
  (if (== OtherActor (Game|GetPlayerCharacter 0))
    (Utilities|FlowControl|DoOnce false
      (:Completed
        ;[0.4977 0.5413 1] Blend to static camera pointing up through the spinning rings...
        (Input|DisableInput (Game|GetPlayerCharacter 0) _returnvalue)
        (Game|Player|SetViewTargetwithBlend _returnvalue (Variables|Default|GetEndCamera) 4.0 "VTBlend_Cubic" 0.0 false)
        (Utilities|FlowControl|Delay 4.0)
        ;[1 0.3088 0.263] Play ending sound...
        (Utilities|PlaySoundifExistsSelf (Variables|Default|GetEndSound))
        ;[0.3322 0.8344 0.5861] Then fade to white...
        (CameraFades|StartCameraFade (Game|GetPlayerCameraManager 0) 0.0 1.0 4.0 "(R=1.000000,G=1.000000,B=1.000000,A=1.000000)" false true)
        ;[1 0.5163 0.3245] And ramp up the FOV as we fade out
        (bind _fov (Timeline|CameraFOVTimeline Play)
          (:Update
            (Camera|SetFieldOfView (Variables|/Script/Engine.CameraActor|GetCameraComponent (Variables|Default|GetEndCamera)) _fov)))))))

(fn ConstructionScript)