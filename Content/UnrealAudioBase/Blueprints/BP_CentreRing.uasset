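; BP_CentreRing is a centre ring actor that rises and starts spinning once both the Garden and Cathedral puzzles are solved.
; GardenSolved and CathedralSolved each count once toward the total, then trigger an attached rotation sound and a timeline that lerps its height from the stored origin to a floating height.
; When the timeline finishes, Tick yaws the ring continuously, applying opposite local offsets around each rotation to compensate for its pivot.
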(event Custom|GardenSolved
  (bind _origposition (Variables|Default|GetOrigPosition))
  (Utilities|FlowControl|DoOnce false
    (:Completed
      (Math|Integer|IncrementInt (Variables|Default|GetNumPuzzlesSolved)
        (:%20%20
          (if (== (Variables|Default|GetNumPuzzlesSolved) 2)
            ;[0.5934 0.6979 1] Trigger ring rotating sound
            (Audio|SpawnSoundAttached (Variables|Default|GetRotatingSound) (Variables|Debug|GetStaticMeshComponent) "None" "0, 0, 0" "0, 0, 0" "KeepRelativeOffset" false 1.0 1.0 0.0 0 0)
            ;[1 0.5843 0.2907] Trigger ring to rise & start rotating once both puzzles have been solved
            (bind _floatindex (Timeline|FloatTimeline Play)
              (:Update
                (Transformation|SetActorLocation (Math|Vector|MakeVector (.x _origposition) (.y _origposition) (Math|Float|Lerp (.z _origposition) (Variables|Default|GetFloatingHeight) _floatindex)) false false))
              (:Finished
                (Variables|Default|SetbRotating true)))))))))

(event Custom|CathedralSolved
  (bind _origposition (Variables|Default|GetOrigPosition))
  (Utilities|FlowControl|DoOnce false
    (:Completed
      (Math|Integer|IncrementInt (Variables|Default|GetNumPuzzlesSolved)
        (:%20%20
          (if (== (Variables|Default|GetNumPuzzlesSolved) 2)
            ;[0.5934 0.6979 1] Trigger ring rotating sound
            (Audio|SpawnSoundAttached (Variables|Default|GetRotatingSound) (Variables|Debug|GetStaticMeshComponent) "None" "0, 0, 0" "0, 0, 0" "KeepRelativeOffset" false 1.0 1.0 0.0 0 0)
            ;[1 0.5843 0.2907] Trigger ring to rise & start rotating once both puzzles have been solved
            (bind _floatindex (Timeline|FloatTimeline Play)
              (:Update
                (Transformation|SetActorLocation (Math|Vector|MakeVector (.x _origposition) (.y _origposition) (Math|Float|Lerp (.z _origposition) (Variables|Default|GetFloatingHeight) _floatindex)) false false))
              (:Finished
                (Variables|Default|SetbRotating true)))))))))

(event EventBeginPlay
  ;[0.4353 1 0.6215] Store ring's original position
  (Variables|Default|SetOrigPosition (Transformation|GetActorLocation)))

(event EventTick
  (params (DeltaSeconds :type Float%20%28single-precision%29))
  (if (Variables|Default|GetbRotating)
    ;[0.5428 0.4555 1] Rotate ring every tick once both puzzles have been solved, offsetting to account for pivot point
    (Transformation|AddActorLocalOffset "700.000000,700.000000,0.000000" false false)
    (Transformation|AddActorLocalRotation (Math|Rotator|MakeRotator 0.0 0.0 (Variables|Default|GetRotateDirection)) false false)
    (Transformation|AddActorLocalOffset "-700.000000,-700.000000,0.000000" false false)))

(fn ConstructionScript)