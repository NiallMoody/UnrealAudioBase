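; Connector Blueprint whose mesh lights up when toggled on and can dim when toggled off.
; BeginPlay creates a dynamic material instance from the static mesh's first material slot.
; ToggleOn plays a timeline that drives that material's Toggle scalar and sets the Toggled flag on finish.
; ToggleOff clears the flag and reverses the same timeline, though a comment marks it as possibly unused.
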(event Custom|ToggleOn
  ;[1 0.2611 0.2392] Light up when toggled on
  (if (not (Variables|Default|GetbToggled))
    (bind _connector_light (Timeline|ConnectorLightTimeline Play)
      (:Update
        (Rendering|Material|SetScalarParameterValue (Variables|Default|GetMaterial) "Toggle" _connector_light :!class /Script/Engine.MaterialInstanceDynamic))
      (:Finished
        (Variables|Default|SetbToggled true)))))

(event Custom|ToggleOff
  ;[0.3952 0.8117 1] Turn off when toggled off (unused?)
  (if (Variables|Default|GetbToggled)
    (Variables|Default|SetbToggled false)
    ;[1 0.2611 0.2392] Light up when toggled on
    (bind _connector_light (Timeline|ConnectorLightTimeline Reverse)
      (:Update
        (Rendering|Material|SetScalarParameterValue (Variables|Default|GetMaterial) "Toggle" _connector_light :!class /Script/Engine.MaterialInstanceDynamic))
      (:Finished
        (Variables|Default|SetbToggled true)))))

(event EventBeginPlay
  ;[0.4328 0.8427 0.521] Store connector's material
  (bind _returnvalue (Rendering|Material|CreateDynamicMaterialInstance (Variables|Debug|GetStaticMeshComponent) 0 0 "None" :!class /Script/Engine.PrimitiveComponent))
  (Variables|Default|SetMaterial _returnvalue))

(fn ConstructionScript)